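; Child enemy Blueprint for the boss Hasan, adding voice lines, facial animation and boss-music control on top of its parent.
; Sound requests play immediately or enter a queue while a line plays, with duration-based timers marking the end.
; Talking drives weighted-random mouth and brow frames through material scalar parameters, while looping timers step eye frames for blinks.
; Other events flag the room camera, play a landing vocal, and change music pitch or fade it on death.
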(event `self.ReceiveBeginPlay`
  (`parent.ReceiveBeginPlay`))

(event `PlayNextQueue`
  (bind _sound_to_play (`self.Sound to Play`))
  (bind _sound_cues_in_queue (`self.Sound Cues in Queue`))
  (bind _sound_cues_in_queue_2 (`self.Sound Cues in Queue`))
  (if (`KismetSystemLibrary.IsValid` (stale `Sound Request` `Sound to Play`)) :!label _label
    (set `self.Sound to Play` (stale `Sound Request` `Sound to Play`)))
  (set `self.Should Add to Queue` (stale `Sound Request` ShouldAddToQueue))
  (if (`KismetSystemLibrary.K2_IsTimerActiveHandle` (`self.LudwigVoice`))
    (if (`self.Should Add to Queue`)
      (for (_array_element _array_index) _sound_cues_in_queue_2
        (`/Engine/EditorBlueprintResources/StandardMacros.IsValid` _array_element
          (:`Is Valid`
            (`KismetArrayLibrary.Array_Add` (`self.Sound Cues in Queue`) _sound_to_play)
            (break))
          (:`Is Not Valid`
            (`KismetArrayLibrary.Array_Set` _sound_cues_in_queue_2 _array_index _sound_to_play)))))
    (else
      (if (not (not (`KismetSystemLibrary.IsValid` (`|GetArrayItem` (`self.Sound Cues in Queue`)))))
        (set `self.Sound to Play` (`|GetArrayItem` _sound_cues_in_queue))
        (`KismetArrayLibrary.Array_Remove` _sound_cues_in_queue))
      (bind _returnvalue (`KismetSystemLibrary.K2_SetTimerDelegate` (`|CreateDelegate` :!event `Sound Has Finished`) (+ (`SoundBase.Duration` (`self.Sound to Play`)) 0.05)))
      (set `self.LudwigVoice` _returnvalue)
      (`GameplayStatics.PlaySoundAtLocation` (`self.Sound to Play`) (`self.K2_GetActorLocation`) (struct) 1.2 1.0 0.0 "/Game/Sounds/A_Loud.A_Loud" null null null)
      (`self.Start Talking`))))

(event `Sound Request`
  (params (`Sound to Play` :type "SoundCue Object Reference") (ShouldAddToQueue :type Boolean))
  (goto _label))

(event `self.SpeedUpMusic`
  (`KismetSystemLibrary.Delay` 2.0)
  (`Timeline|AdjustPitch` :!via `PlayFromStart`
    (:`Update`
      (`AudioComponent.SetPitchMultiplier` (`/Game/Sounds/BossMusic.AudioBossMusic` (`self.TheMusic`)) 1.4))))

(event `Sound Has Finished`
  (`KismetSystemLibrary.K2_ClearAndInvalidateTimerHandle` (`self.TalkingTimer_0`))
  (`MeshComponent.SetScalarParameterValueOnMaterials` (`self.Mesh`) "MouthSpecificFrame" 1.0)
  (`MeshComponent.SetScalarParameterValueOnMaterials` (`self.Mesh`) "BrowsSpecificFrame" 1.0)
  (if (`KismetSystemLibrary.IsValid` (`|GetArrayItem` (`self.Sound Cues in Queue`)))
    (`KismetSystemLibrary.Delay` 0.1)
    (`self.PlayNextQueue`)))

(event `SetPitchBackTO0`
  (`AudioComponent.SetPitchMultiplier` (`/Game/Sounds/BossMusic.AudioBossMusic` (`self.TheMusic`)) 1.0))

(event `/Game/Enemies/HasanShakeInterface.IShook`
  (`self.Sound Request` "/Game/Sounds/DialogueRawFiles/Hasan/Hasan_LandingVocal_1_Cue.Hasan_LandingVocal_1_Cue" true))

(event `Start Talking`
  (bind _returnvalue (`KismetSystemLibrary.K2_SetTimerDelegate` (`|CreateDelegate` :!event `Change Vizeme`) 0.125 true))
  (set `self.TalkingTimer_0` _returnvalue))

(event `Change Vizeme`
  (bind _returnvalue (`KismetMathLibrary.RandomInteger` 100))
  (`|ExecutionSequence`
    (:`then_0`
      (if (<= _returnvalue 24)
        (set `self.CurrentVisemeInTalkingSequence_0` 2.0)
        (elif (<= _returnvalue 26)
          (set `self.CurrentVisemeInTalkingSequence_0` 8.0)
          (elif (<= _returnvalue 15)
            (set `self.CurrentVisemeInTalkingSequence_0` 7.0)
            (elif (<= _returnvalue 7)
              (set `self.CurrentVisemeInTalkingSequence_0` 3.0)
              (elif (<= _returnvalue 7)
                (set `self.CurrentVisemeInTalkingSequence_0` 4.0)
                (elif (<= _returnvalue 4)
                  (set `self.CurrentVisemeInTalkingSequence_0` 5.0)
                  (elif (<= _returnvalue 4)
                    (set `self.CurrentVisemeInTalkingSequence_0` 6.0)
                    (elif (<= _returnvalue 4)
                      (set `self.CurrentVisemeInTalkingSequence_0` 9.0)
                      (elif (<= _returnvalue 3)
                        (set `self.CurrentVisemeInTalkingSequence_0` 10.0)
                        (else
                          (set `self.CurrentVisemeInTalkingSequence_0` 11.0)))))))))))
      (`MeshComponent.SetScalarParameterValueOnMaterials` (`self.Mesh`) "MouthSpecificFrame" (`self.CurrentVisemeInTalkingSequence_0`)))
    (:`then_1`
      (if (<= _returnvalue 25)
        (set `self.CurrentBrows_0` 2.0)
        (else
          (set `self.CurrentBrows_0` 1.0)))
      (`MeshComponent.SetScalarParameterValueOnMaterials` (`self.Mesh`) "BrowsSpecificFrame" (`self.CurrentBrows_0`)))))

(event `self.HasanDiedToChild`
  (`AudioComponent.FadeOut` (`/Game/Sounds/BossMusic.AudioBossMusic` (`self.TheMusic`)) 5.0 0.0 "Linear"))

(event `self.HasanSpecialEvent`
  (set `/Game/ThirdPerson/Blueprints/Camera/BP_Cam_Master.InHasansRoom` true (`self.TheRoomCam`))
  (`self.Begin Blinking Loop`))

(event `Begin Blinking Loop_Fresh`
  (`KismetSystemLibrary.K2_SetTimerDelegate` (`|CreateDelegate` :!event `SendBlinkEvent`) 5.0 true))

(event `SendBlinkEvent`
  (bind _returnvalue (`KismetSystemLibrary.K2_SetTimerDelegate` (`|CreateDelegate` :!event `ChangeBlinkFrame`) 0.125 true))
  (set `self.BlinkingFramesTimer_0` _returnvalue))

(event `ChangeBlinkFrame`
  (bind _currenteyesframe_0 (`self.CurrentEyesFrame_0`))
  (`MeshComponent.SetScalarParameterValueOnMaterials` (`self.Mesh`) "EyesSpecificFrame" (select `int` (`self.CurrentEyesFrame_0`) :`0` 1.0 :`1` 2.0 :`2` 3.0 :`3` 2.0 :`4` 1.0 :!type "Float (single-precision)"))
  (if (!= _currenteyesframe_0 4)
    (`/Engine/EditorBlueprintResources/StandardMacros.IncrementInt` _currenteyesframe_0)
    (else
      (`KismetSystemLibrary.K2_ClearAndInvalidateTimerHandle` (`self.BlinkingFramesTimer_0`))
      (set `self.CurrentEyesFrame_0` 0))))

(fn `Play Next in Queue`)

(fn `UserConstructionScript`
  (`parent.UserConstructionScript`))