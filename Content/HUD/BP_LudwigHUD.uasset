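; BP_LudwigHUD is a HUD actor that follows the first player's camera.
; Every Tick it copies the camera manager's location and rotation onto itself, without sweep or teleport.
; An unconnected debug sphere draw, offset along the camera's forward vector by CamCenterExtent, never runs.
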(event `self.ReceiveTick`
  (params (DeltaSeconds :type "Float (single-precision)"))
  (bind _returnvalue (`GameplayStatics.GetPlayerCameraManager` 0))
  (`self.K2_SetActorLocation` (`PlayerCameraManager.GetCameraLocation` _returnvalue))
  (`self.K2_SetActorRotation` (`PlayerCameraManager.GetCameraRotation` _returnvalue)))

(fn `UserConstructionScript`)